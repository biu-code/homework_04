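; BP_M16 is an M16 weapon Blueprint that provides firing effects, a muzzle transform and an ammo counter.
; KaiHuo (fire) spawns a LiZi (particle) actor at the Arrow component's transform with a short lifespan.
; GetZiDanLocation exposes that transform as the bullet origin.
; ZiDan decrements ZiDanLiang while ammo remains but returns true even when empty, and KaiHuo does not call it.
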(event Custom|KaiHuo
  (bind _returnvalue (Game|SpawnActorfromClass "/Game/M16/Blueprint/LiZi.LiZi_C" (Transformation|GetWorldTransform (Variables|Default|GetArrow)) "Undefined" 0 0))
  (Actor|SetLifeSpan _returnvalue 3.0))

(fn ConstructionScript)

(fn GetZiDanLocation
  (return (Transformation|GetWorldTransform (Variables|Default|GetArrow))))

(fn ZiDan
  (if (> (Variables|Default|GetZiDanLiang) 0)
    (Variables|Default|SetZiDanLiang (- (Variables|Default|GetZiDanLiang) 1))
    (return true)
    (else
      (return true))))