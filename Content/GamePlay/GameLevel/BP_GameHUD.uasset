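; BP_GameHUD is the game HUD Blueprint that manages the on-screen widgets for a shooter level.
; On BeginPlay it adds the main UI and an AI count (AIShuLiang) widget to the viewport.
; Paired events show and remove the aiming crosshair (ZhunXing) and reload (TianJiaZiDan) widgets.
; These two are created on first use, then cached and reused on later calls.
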(event Custom|KaiJIng
  (Utilities|IsValid (Variables|Default|GetZhunXing)
    (:Is%20Valid
      _)
    (:Is%20Not%20Valid
      (bind _returnvalue (UserInterface|CreateWidget "/Game/UI/ZhunXing.ZhunXing_C"))
      (bind _output_get (Variables|Default|SetZhunXing _returnvalue))))
  (UserInterface|Viewport|AddtoViewport _output_get 0))

(event Custom|RemoveKaiJing
  (bind _zhunxing (Variables|Default|GetZhunXing))
  (Utilities|IsValid _zhunxing
    (:Is%20Valid
      (Widget|RemovefromParent _zhunxing))))

(event Custom|HuanDan
  (Utilities|IsValid (Variables|Default|GetHuanDanUi)
    (:Is%20Valid
      _)
    (:Is%20Not%20Valid
      (bind _returnvalue (UserInterface|CreateWidget "/Game/UI/TianJiaZiDan.TianJiaZiDan_C" (Game|Player|GetOwningPlayerController)))
      (bind _output_get (Variables|Default|SetHuanDanUi _returnvalue))))
  (UserInterface|Viewport|AddtoViewport _output_get 0))

(event Custom|HuanDanRemove
  (bind _huandanui (Variables|Default|GetHuanDanUi))
  (Utilities|IsValid _huandanui
    (:Is%20Valid
      (Widget|RemovefromParent _huandanui))))

(event EventBeginPlay
  (bind _returnvalue (UserInterface|CreateWidget "/Game/UI/MainUI.MainUI_C" (Game|Player|GetOwningPlayerController)))
  (bind _output_get (Variables|Default|SetMainUI _returnvalue))
  (UserInterface|Viewport|AddtoViewport _output_get 0)
  (bind _returnvalue_2 (UserInterface|CreateWidget "/Game/UI/AIShuLiang.AIShuLiang_C"))
  (UserInterface|Viewport|AddtoViewport _returnvalue_2 0))

(fn ConstructionScript)