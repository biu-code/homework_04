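; BP_ZiDan is a bullet actor that damages AI_Energy enemies on contact.
; It plays a sound effect on BeginPlay; overlapping an AI_Energy with its ZiDan component calls ShouShang with fixed damage, then destroys the bullet.
; The construction script casts the root component's owner, the actor itself, to BP_GamePawn, and only on success rotates the root toward the GetZhengXiangLiang vector.
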(event OnComponentBeginOverlap(ZiDan)
  (params (OverlappedComponent :type Primitive%20Component%20Object%20Reference) (OtherActor :type Actor%20Object%20Reference) (OtherComp :type Primitive%20Component%20Object%20Reference) (OtherBodyIndex :type Integer) (bFromSweep :type Boolean) (SweepResult :type Hit%20Result%20Structure%20%28by%20ref%29))
  (Utilities|IsValid self
    (:Is%20Valid
      (bind _asai_energy (Utilities|Casting|CastToAI_Energy OtherActor))
      (Default|ShouShang _asai_energy 1e+01)
      (Actor|DestroyActor))))

(event EventBeginPlay
  (Audio|PlaySound2D (Variables|Default|GetYinXiao) 1.0 1.0 0.0 0 0))

(fn ConstructionScript
  (bind _asbp_game_pawn (Utilities|Casting|CastToBP_GamePawn (Components|GetOwner (Variables|Default|GetDefaultSceneRoot))))
  (Transformation|SetWorldRotation (Variables|Default|GetDefaultSceneRoot) (Math|Rotator|FindLookatRotation (Transformation|GetWorldLocation (Variables|Default|GetDefaultSceneRoot)) (Default|GetZhengXiangLiang _asbp_game_pawn)) false false))